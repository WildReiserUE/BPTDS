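; Armor pickup that adds a fixed amount of armor to a BP_TDS_Character that overlaps its box.
; It adds a rotating movement component on BeginPlay.
; If armor is already full, it shows a max-armor widget with a warning sound and stays in the world.
; Otherwise it adds armor without clamping, shows feedback, removes the box and rune components, then destroys itself after a short delay.
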(event `self.ReceiveBeginPlay`
  ;[1 1 1] EventbeginePlay (AddRotatingMovementComponent)
  (`AddComponent|NODE_AddRotatingMovementComponent-0`))

(event `self.Box.OnComponentBeginOverlap`
  (params (OverlappedComponent :type "PrimitiveComponent Object Reference") (OtherActor :type "Actor Object Reference") (OtherComp :type "PrimitiveComponent Object Reference") (OtherBodyIndex :type Integer) (bFromSweep :type Boolean) (SweepResult :type "HitResult Structure (by ref)"))
  ;[1 1 1] Pick Up Armor
  (bind _asbp_tds_character (cast `/Game/TDS_Starter_Pack/Blueprints/BP_TDS_Character` OtherActor))
  (if (>= (`/Game/TDS_Starter_Pack/Blueprints/BP_TDS_Character.Armor` _asbp_tds_character) 100.0)
    (bind _returnvalue (`|CreateWidget` "/Game/TDS_Starter_Pack/Widgets/BP_YouHaveMaxArmorWidget.BP_YouHaveMaxArmorWidget_C"))
    (`UserWidget.AddToViewport` _returnvalue 0)
    (`AudioComponent.Play` (`self.Warning_Cue`) 0.0)
    (else
      (set `/Game/TDS_Starter_Pack/Blueprints/BP_TDS_Character.Armor` (+ (`/Game/TDS_Starter_Pack/Blueprints/BP_TDS_Character.Armor` _asbp_tds_character) 25.0) _asbp_tds_character)
      (`KismetSystemLibrary.PrintString` "+Armor" true true (struct :`R` 0.298948 :`G` 1.0 :`B` 0.123761 :`A` 1.0))
      (`ActorComponent.K2_DestroyComponent` (`self.Box`))
      (`AudioComponent.Play` (`self.PickUpRandom_Cue`) 0.0)
      (bind _returnvalue_2 (`|CreateWidget` "/Game/TDS_Starter_Pack/Widgets/BP_+Armor_Widget.BP_+Armor_Widget_C"))
      (`UserWidget.AddToViewport` _returnvalue_2 0)
      (`ActorComponent.K2_DestroyComponent` (`self.Rune_P1`))
      (`KismetSystemLibrary.Delay` 1.0)
      (`self.K2_DestroyActor`))))

(fn `UserConstructionScript`)