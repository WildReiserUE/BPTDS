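; BP_GunPickUp is a spinning gun pickup that arms BP_TDS_Character when it overlaps the Box.
; BeginPlay adds a rotating movement component.
; On overlap it enables the character's gun flags, plays a random pickup cue, removes its own box and mesh, and shows the character's gun.
; It then clears all widgets, creates the gun ammo and HUD widgets, and destroys itself after a short delay.
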(event `self.ReceiveBeginPlay`
  ;[1 1 1] EventbeginePlay (AddRotatingMovementComponent)
  (`AddComponent|NODE_AddRotatingMovementComponent-0`))

(event `self.Box.OnComponentBeginOverlap`
  (params (OverlappedComponent :type "PrimitiveComponent Object Reference") (OtherActor :type "Actor Object Reference") (OtherComp :type "PrimitiveComponent Object Reference") (OtherBodyIndex :type Integer) (bFromSweep :type Boolean) (SweepResult :type "HitResult Structure (by ref)"))
  ;[1 1 1] Pick Up  Gun
  (bind _asbp_tds_character (cast `/Game/TDS_Starter_Pack/Blueprints/BP_TDS_Character` OtherActor))
  (bind _output_get (set `self.Char` _asbp_tds_character))
  (set `/Game/TDS_Starter_Pack/Blueprints/BP_TDS_Character.InteractionGun` true _output_get)
  (set `/Game/TDS_Starter_Pack/Blueprints/BP_TDS_Character.UseGun` true (`self.Char`))
  (`AudioComponent.Play` (`self.PickUpRandom_Cue`) 0.0)
  (`ActorComponent.K2_DestroyComponent` (`self.Box`))
  (`ActorComponent.K2_DestroyComponent` (`self.SK_FPGunBlue`))
  (`SceneComponent.SetVisibility` (`/Game/TDS_Starter_Pack/Blueprints/BP_TDS_Character.Gun` (`self.Char`)) true false)
  (`WidgetLayoutLibrary.RemoveAllWidgets`)
  (bind _returnvalue (`|CreateWidget` "/Game/TDS_Starter_Pack/Widgets/BP_GunAmmoWidget.BP_GunAmmoWidget_C"))
  (`UserWidget.AddToViewport` _returnvalue 0)
  (bind _returnvalue_2 (`|CreateWidget` "/Game/TDS_Starter_Pack/Widgets/BP_HUD_Widget.BP_HUD_Widget_C"))
  (`UserWidget.AddToViewport` _returnvalue_2 0)
  (`KismetSystemLibrary.Delay` 1.0)
  (`self.K2_DestroyActor`))

(fn `UserConstructionScript`)