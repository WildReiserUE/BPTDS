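; BP_HealthPickUp is a health pickup actor for the top-down shooter character BP_TDS_Character, triggered by overlapping its Box component.
; Below 100 health, it adds 25 without clamping, plays a sound, shows a health widget, removes its text, box and particle components, then destroys itself after a short delay.
; At full health, it stays in place and shows a max-health widget with a warning sound.
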(event `self.ReceiveBeginPlay`
  ;[1 1 1] EventbeginePlay (AddRotatingMovementComponent)
)

(event `self.Box.OnComponentBeginOverlap`
  (params (OverlappedComponent :type "PrimitiveComponent Object Reference") (OtherActor :type "Actor Object Reference") (OtherComp :type "PrimitiveComponent Object Reference") (OtherBodyIndex :type Integer) (bFromSweep :type Boolean) (SweepResult :type "HitResult Structure (by ref)"))
  ;[1 1 1] Pick Up Health
  (bind _asbp_tds_character (cast `/Game/TDS_Starter_Pack/Blueprints/BP_TDS_Character` OtherActor))
  (if (>= (`/Game/TDS_Starter_Pack/Blueprints/BP_TDS_Character.Health` _asbp_tds_character) 100.0)
    (bind _returnvalue (`|CreateWidget` "/Game/TDS_Starter_Pack/Widgets/BP_YouHaveMaxhealth_Widget.BP_YouHaveMaxhealth_Widget_C"))
    (`UserWidget.AddToViewport` _returnvalue 0)
    (`AudioComponent.Play` (`self.Warning_Cue`) 0.0)
    (else
      (set `/Game/TDS_Starter_Pack/Blueprints/BP_TDS_Character.Health` (+ (`/Game/TDS_Starter_Pack/Blueprints/BP_TDS_Character.Health` _asbp_tds_character) 25.0) _asbp_tds_character)
      (`KismetSystemLibrary.PrintString` "+Health" true true (struct :`R` 0.298948 :`G` 1.0 :`B` 0.123761 :`A` 1.0))
      (`ActorComponent.K2_DestroyComponent` (`self.TextRender`))
      (`ActorComponent.K2_DestroyComponent` (`self.Box`))
      (`AudioComponent.Play` (`self.PickUpRandom_Cue`) 0.0)
      (bind _returnvalue_2 (`|CreateWidget` "/Game/TDS_Starter_Pack/Widgets/BP_+Health_Widget.BP_+Health_Widget_C"))
      (`UserWidget.AddToViewport` _returnvalue_2 0)
      (`ActorComponent.K2_DestroyComponent` (`self.Rune_And_RIngs_Green_P`))
      (`KismetSystemLibrary.Delay` 1.0)
      (`self.K2_DestroyActor`))))

(fn `UserConstructionScript`)