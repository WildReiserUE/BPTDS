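; BP_BuildingShelter is a building that can turn its roof transparent while a top-down shooter character is inside.
; When TransRoof is enabled, a BP_TDS_Character overlapping the Box swaps the Roof's first material slot to glass.
; Ending the overlap sets a hard-coded walnut wood material rather than caching the original.
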(event `self.Box.OnComponentBeginOverlap`
  (params (OverlappedComponent :type "PrimitiveComponent Object Reference") (OtherActor :type "Actor Object Reference") (OtherComp :type "PrimitiveComponent Object Reference") (OtherBodyIndex :type Integer) (bFromSweep :type Boolean) (SweepResult :type "HitResult Structure (by ref)"))
  ;[1 1 1] When a player enters the building (overlap the collision box), the glass material is applied to the roof so that the roof becomes transparent.
  (if (`self.bTransRoof`)
    (cast `/Game/BaseTDS/Blueprints/BP_TDS_Character` OtherActor)
    (`PrimitiveComponent.SetMaterial` (`self.Roof`) 0 "/Game/BaseTDS/ExampleContent/StarterContent/Materials/M_Glass.M_Glass")))

(event `self.Box.OnComponentEndOverlap`
  (params (OverlappedComponent :type "PrimitiveComponent Object Reference") (OtherActor :type "Actor Object Reference") (OtherComp :type "PrimitiveComponent Object Reference") (OtherBodyIndex :type Integer))
  ;[1 1 1] When a player leaves the building (end overlap the box), the material that was on it is applied to the roof before.
  (if (`self.bTransRoof`)
    (cast `/Game/BaseTDS/Blueprints/BP_TDS_Character` OtherActor)
    (`PrimitiveComponent.SetMaterial` (`self.Roof`) 0 "/Game/BaseTDS/ExampleContent/StarterContent/Materials/M_Wood_Walnut.M_Wood_Walnut")))

(fn `UserConstructionScript`)